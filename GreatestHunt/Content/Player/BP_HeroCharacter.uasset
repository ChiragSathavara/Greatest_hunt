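; BP_HeroCharacter is the player character Blueprint, handling HUD setup and input for inventory, lock-on and exit.
; BeginPlay adds the player health widget to the viewport, while Tick prints the current Health on screen as text.
; Enhanced Input actions open a new inventory widget with cursor and UI-only input, toggle targeting through LockonComp, or load the MainMenu level.
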(event `self.ReceiveBeginPlay`
  (bind _returnvalue (`|CreateWidget` "/Game/Widgetss/WB_PlayerHealth.WB_PlayerHealth_C" (`GameplayStatics.GetPlayerController` 0)))
  (`UserWidget.AddToViewport` _returnvalue 0))

(event `self.ReceiveTick`
  (params (DeltaSeconds :type "Float (single-precision)"))
  (`KismetSystemLibrary.PrintText` (`|FormatText` "Player health is {Health}" (`self.Health`)) true false (struct :`G` 0.66 :`B` 1.0 :`A` 1.0) 0.0))

(event `EnhancedInput|/Game/Player/Inputs/IA_Tab`
  (params (ActionValue :type Boolean) (ElapsedSeconds :type "Float (double-precision)") (TriggeredSeconds :type "Float (double-precision)") (InputAction :type "InputAction Object Reference" :default "/Game/Player/Inputs/IA_Tab.IA_Tab"))
  (bind _returnvalue (`GameplayStatics.GetPlayerController` 0))
  (:`Started`
    (bind _returnvalue_2 (`|CreateWidget` "/Game/Widgetss/WB_Inventory.WB_Inventory_C" _returnvalue))
    (`UserWidget.AddToViewport` _returnvalue_2 0)
    (set `PlayerController.bShowMouseCursor` true _returnvalue)
    (`WidgetBlueprintLibrary.SetInputMode_UIOnlyEx` _returnvalue _returnvalue_2 "DoNotLock" true)))

(event `EnhancedInput|/Game/Player/Inputs/IA_Lock`
  (params (ActionValue :type Boolean) (ElapsedSeconds :type "Float (double-precision)") (TriggeredSeconds :type "Float (double-precision)") (InputAction :type "InputAction Object Reference" :default "/Game/Player/Inputs/IA_Lock.IA_Lock"))
  (:`Started`
    (`LockonComponent.ToggleLockOn` (`self.LockonComp`) 750.0)))

(event `EnhancedInput|/Game/Player/Inputs/IA_EXIT`
  (params (ActionValue :type Boolean) (ElapsedSeconds :type "Float (double-precision)") (TriggeredSeconds :type "Float (double-precision)") (InputAction :type "InputAction Object Reference" :default "/Game/Player/Inputs/IA_EXIT.IA_EXIT"))
  (:`Started`
    (`GameplayStatics.OpenLevel` "MainMenu")))

(fn `UserConstructionScript`)